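; BP_MonitorPawn is a pawn that smoothly animates changes to its zoom scale.
; On ZoomScaleChanged, it stores the current scale, computes and debug-prints an offset from the input, then plays ZoomTimeline to apply that offset over the starting value.
; An IsZooming flag ignores new zoom requests until the timeline finishes.
; The zoom getter, setter and offset calculation are defined outside this file.
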(event `self.ZoomScaleChanged`
  (params (InZoomScale :type "Float (single-precision)"))
  (if (not (`self.IsZooming`))
    (`|ExecutionSequence`
      (:`then_0`
        ;[1 1 1] Set Parameter
        (set `self.IsZooming` true)
        (set `self.EarlyZoomScale` (`self.GetZoomScale`))
        (bind _output_get (set `self.OffsetZoomScale` (`self.GetOffsetZoomScale` InZoomScale)))
        (`KismetSystemLibrary.PrintString` (`KismetStringLibrary.Conv_DoubleToString` _output_get)))
      (:`then_1`
        ;[1 1 1] Execute Zoom
        (bind (_direction _zoom) (`Timeline|ZoomTimeline` :!via `PlayFromStart`)
          (:`Update`
            (`self.SetZoomScale` (+ (* _zoom (`self.OffsetZoomScale`)) (`self.EarlyZoomScale`))))
          (:`Finished`
            (set `self.IsZooming` false)))))))

(fn `UserConstructionScript`)